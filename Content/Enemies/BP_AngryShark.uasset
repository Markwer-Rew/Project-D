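; Angry shark enemy that wanders the navmesh and damages the first-person character heavily when its box overlaps them.
; Random AI moves chain on success to form the roaming loop.
; Pawn sensing by sight or hearing triggers a faster chase toward the seen pawn, using DoOnce to switch animation and speed once.
; A retriggerable delay restores slower roaming and re-arms the chase shortly after sensing stops.
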(event `self.Box.OnComponentBeginOverlap`
  (params (OverlappedComponent :type "PrimitiveComponent Object Reference") (OtherActor :type "Actor Object Reference") (OtherComp :type "PrimitiveComponent Object Reference") (OtherBodyIndex :type Integer) (bFromSweep :type Boolean) (SweepResult :type "HitResult Structure (by ref)"))
  ; Chase/Kill Logic
  (bind _asbp_first_person_character (cast `/Game/FirstPerson/Blueprints/BP_FirstPersonCharacter` OtherActor))
  (`GameplayStatics.ApplyDamage` _asbp_first_person_character 100.0))

(event `self.ReceiveBeginPlay`
  ; Chase/Kill Logic
  (`self.MoveToRandomLocation`))

(event `MoveToRandomLocation`
  ; Chase/Kill Logic
  (bind _randomlocation (`NavigationSystemV1.K2_GetRandomLocationInNavigableRadius` (`self.K2_GetActorLocation`) 600.0 null null))
  (`|AIMoveTo` self _randomlocation null
    (:`OnSuccess`
      (`self.MoveToRandomLocation`))))

(event `CanChaseAgain`
  ; Chase/Kill Logic
  (goto _label_2 :!via `Reset`))

(event `self.PawnSensing.OnHearNoise`
  (params (Instigator :type "Pawn Object Reference") (Location :type "Vector Structure (by ref)") (Volume :type "Float (single-precision)"))
  ; Chase/Kill Logic
  (`|ExecutionSequence` :!label _label
    (:`then_0`
      (`/Engine/EditorBlueprintResources/StandardMacros.DoOnce` false :!label _label_2
        (:`Completed`
          (`SkeletalMeshComponent.PlayAnimation` (`self.Mesh`) null true)
          (set `CharacterMovementComponent.MaxWalkSpeed` 250.0 (`self.CharacterMovement`)))))
    (:`then_1`
      (`|AIMoveTo` self (0.0 0.0 0.0) (stale `self.PawnSensing.OnSeePawn` Pawn)
        (:`then`
          (`KismetSystemLibrary.RetriggerableDelay` 1.5)
          (`SkeletalMeshComponent.PlayAnimation` (`self.Mesh`) null true)
          (set `CharacterMovementComponent.MaxWalkSpeed` 150.0 (`self.CharacterMovement`))
          (`self.CanChaseAgain`)
          (`self.MoveToRandomLocation`))))))

(event `self.PawnSensing.OnSeePawn`
  (params (Pawn :type "Pawn Object Reference"))
  ; Chase/Kill Logic
  (goto _label))

(fn `UserConstructionScript`)