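; Box trigger zone that raises the player character's Davlenie (pressure) while overlapped and lowers it after exit.
; Any overlap begin or end starts a looping timer that, with delays, changes player 0's value in fixed steps.
; The increase stops at a cap, while the decrease has no floor.
; Each overlap event sets the opposing timer handle to None before clearing it, so that timer is never actually cancelled.
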(event `self.Box.OnComponentBeginOverlap`
  (params (OverlappedComponent :type "PrimitiveComponent Object Reference") (OtherActor :type "Actor Object Reference") (OtherComp :type "PrimitiveComponent Object Reference") (OtherBodyIndex :type Integer) (bFromSweep :type Boolean) (SweepResult :type "HitResult Structure (by ref)"))
  ; UpOfDavlenie
  (bind _output_get (set `self.TimerStopPressure` (struct)))
  (`KismetSystemLibrary.K2_ClearAndInvalidateTimerHandle` _output_get)
  (bind _returnvalue (`KismetSystemLibrary.K2_SetTimerDelegate` (delegate `MakeMorePressure`) 1.0 true))
  (set `self.TimerMakingPressure` _returnvalue))

(event `MakeMorePressure`
  ; UpOfDavlenie
  (bind _asbp_first_person_character (cast `/Game/FirstPerson/Blueprints/BP_FirstPersonCharacter` (`GameplayStatics.GetPlayerCharacter` 0)))
  (bind _davlenie (`/Game/FirstPerson/Blueprints/BP_FirstPersonCharacter.Davlenie` _asbp_first_person_character))
  (if (not (>= _davlenie 20.0))
    (`KismetSystemLibrary.Delay` 1.0)
    (set `/Game/FirstPerson/Blueprints/BP_FirstPersonCharacter.Davlenie` (+ _davlenie 2.0) _asbp_first_person_character)))

(event `StopMakePressure`
  ; FallOfDavlenie
  (bind _asbp_first_person_character (cast `/Game/FirstPerson/Blueprints/BP_FirstPersonCharacter` (`GameplayStatics.GetPlayerCharacter` 0)))
  (`KismetSystemLibrary.Delay` 1.0)
  (set `/Game/FirstPerson/Blueprints/BP_FirstPersonCharacter.Davlenie` (- (`/Game/FirstPerson/Blueprints/BP_FirstPersonCharacter.Davlenie` _asbp_first_person_character) 2.0) _asbp_first_person_character)
  (`KismetSystemLibrary.Delay` 2.0))

(event `self.Box.OnComponentEndOverlap`
  (params (OverlappedComponent :type "PrimitiveComponent Object Reference") (OtherActor :type "Actor Object Reference") (OtherComp :type "PrimitiveComponent Object Reference") (OtherBodyIndex :type Integer))
  ; FallOfDavlenie
  (bind _output_get (set `self.TimerMakingPressure` (struct)))
  (`KismetSystemLibrary.K2_ClearAndInvalidateTimerHandle` _output_get)
  (bind _returnvalue (`KismetSystemLibrary.K2_SetTimerDelegate` (delegate `StopMakePressure`) 1.0 true))
  (set `self.TimerStopPressure` _returnvalue))

(fn `UserConstructionScript`)