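; BP_Note_Child is a note variant that ends the game when the player interacts with it.
; A one-shot Interact plays a cable-up sound, disables movement, clears the character's notes and game-active flag, and starts the HUD end-screen animation.
; A looping timer then repeatedly raises the player's capsule from its saved position, lifting the player steadily upward.
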(event `self.ReceiveBeginPlay`
  (`|ExecutionSequence`
    (:`then_0`
      (bind _asbp_first_person_character (cast `/Game/FirstPerson/Blueprints/BP_FirstPersonCharacter` (`GameplayStatics.GetPlayerCharacter` 0)))
      (set `self.As BP First Person Character` _asbp_first_person_character))))

(event `/Game/Blueprints/BPI_Interact.Interact`
  (bind _as_bp_first_person_character (`self.As BP First Person Character`))
  (bind _endscreen (`/Game/UI/BP_MainHUD.EndScreen` (`/Game/FirstPerson/Blueprints/BP_FirstPersonCharacter.HUD` (`self.As BP First Person Character`))))
  (`/Engine/EditorBlueprintResources/StandardMacros.DoOnce` false
    (:`Completed`
      (`GameplayStatics.PlaySound2D` "/Game/Sound/S_CableUp_Cue.S_CableUp_Cue" 1.0 1.0 0.0 null null)
      (set `self.WorldLocation` (`SceneComponent.K2_GetComponentLocation` (`Character.CapsuleComponent` (`self.As BP First Person Character`))))
      (`CharacterMovementComponent.DisableMovement` (`Character.CharacterMovement` _as_bp_first_person_character))
      (set `/Game/FirstPerson/Blueprints/BP_FirstPersonCharacter.TheGameISActive` false _as_bp_first_person_character)
      (`KismetArrayLibrary.Array_Clear` (`/Game/FirstPerson/Blueprints/BP_FirstPersonCharacter.Notes` _as_bp_first_person_character))
      (`KismetSystemLibrary.K2_SetTimerDelegate` (delegate `WIN`) 0.1 true)
      (`UserWidget.PlayAnimation` _endscreen (`/Game/UI/WBP_EndScreen.End` _endscreen) 0.0 1 "Forward" 1.0 false))))

(event `WIN`
  (bind (_worldlocation_x _worldlocation_y _worldlocation_z) (`KismetMathLibrary.BreakVector` (`self.WorldLocation`)))
  (bind _output_get (set `self.WorldLocation` (`KismetMathLibrary.MakeVector` _worldlocation_x _worldlocation_y (+ _worldlocation_z 3.0))))
  (`SceneComponent.K2_SetRelativeLocation` (`Character.CapsuleComponent` (`self.As BP First Person Character`)) (`KismetMathLibrary.MakeVector` (.x _output_get) (.y _output_get) (.z _output_get)) false false))

(fn `UserConstructionScript`
  (`parent.UserConstructionScript`))